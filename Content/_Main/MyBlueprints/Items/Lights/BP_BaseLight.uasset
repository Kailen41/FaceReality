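; Base light actor that works as a point, spot or rect light, with on/off events and randomised flicker effects.
; Construction script and on/off events toggle component visibility from LightType and IsLightOn.
; BeginPlay and TurnonLights start a looping timer that drives Flicker, Fade or a random mix of both.
; DoOnce gates with random delays pace the intensity changes, using hard 0/2000 switches for flicker and timelines for fades.
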(event Custom|LightFlicker
  (bind _returnvalue (Utilities|Time|SetTimerbyEvent (delegate Custom|LightFlickerTimer) 0.1 true))
  (Variables|Default|SetFlickerTimerHandle _returnvalue))

(event Custom|LightFlickerTimer
  (switch Utilities|FlowControl|Switch|SwitchonE_FlickerType (Variables|Default|GetLightFlickerType)
    (:NewEnumerator1
      ;[1 0 1] Flicker
      (Utilities|FlowControl|DoOnce false :!label _label
        (:Completed
          (if (Math|Random|RandomBool)
            (Rendering|Components|Light|SetIntensity (Variables|Default|GetSpotLight) 0.0)
            (Variables|Default|SetCurrentIntensity 0.0)
            (else
              (Rendering|Components|Light|SetIntensity (Variables|Default|GetSpotLight) 2e+03)
              (Variables|Default|SetCurrentIntensity 2e+03)))
          (Utilities|FlowControl|Delay (Math|Random|RandomFloatinRange 0.0 0.3))
          (goto _label Reset))))
    (:NewEnumerator2
      ;[1 0 1] Fade
      (Utilities|FlowControl|DoOnce false :!label _label_2
        (:Completed
          (if (== (Variables|Default|GetCurrentIntensity) (Variables|Default|GetMaxLightIntensity))
            (Components|Timeline|SetTimelineLength (Variables|Default|GetFadeTo0_TL) (Math|Random|RandomFloatinRange 0.1 0.6))
            (bind _lightintensity_alpha (Timeline|FadeTo0_TL PlayFromStart)
              (:Update
                (Rendering|Components|Light|SetIntensity (Variables|Default|GetSpotLight) _lightintensity_alpha)
                (Variables|Default|SetCurrentIntensity 0.0))
              (:Finished
                (Utilities|FlowControl|Delay (Math|Random|RandomFloatinRange 0.0 0.6) :!label _label_3)
                (goto _label_2 Reset)))
            (else
              (Components|Timeline|SetTimelineLength (Variables|Default|GetFadeToLit_TL) (Math|Random|RandomFloatinRange 0.1 0.6))
              (bind _lightintensity_alpha_2 (Timeline|FadeToLit_TL PlayFromStart)
                (:Update
                  (Rendering|Components|Light|SetIntensity (Variables|Default|GetSpotLight) _lightintensity_alpha_2)
                  (Variables|Default|SetCurrentIntensity (Variables|Default|GetMaxLightIntensity)))
                (:Finished
                  (goto _label_3))))))))
    (:NewEnumerator3
      (if (Math|Random|RandomBool)
        ;[1 0 1] Flicker
        (if (not (Variables|Default|GetIsFadeActive?))
          (Utilities|FlowControl|DoOnce false :!label _label_4
            (:Completed
              (if (Math|Random|RandomBool)
                (Rendering|Components|Light|SetIntensity (Variables|Default|GetSpotLight) 0.0)
                (Variables|Default|SetCurrentIntensity 0.0)
                (else
                  (Rendering|Components|Light|SetIntensity (Variables|Default|GetSpotLight) 2e+03)
                  (Variables|Default|SetCurrentIntensity 2e+03)))
              (Utilities|FlowControl|Delay (Math|Random|RandomFloatinRange 0.0 0.3))
              (goto _label_4 Reset))))
        (else
          ;[1 0 1] Fade
          (Utilities|FlowControl|DoOnce false :!label _label_5
            (:Completed
              (if (== (Variables|Default|GetCurrentIntensity) (Variables|Default|GetMaxLightIntensity))
                (Components|Timeline|SetTimelineLength (Variables|Default|GetFadeTo0_TL) (Math|Random|RandomFloatinRange 0.1 0.6))
                (bind _lightintensity_alpha_3 (Timeline|Timeline PlayFromStart)
                  (:Update
                    (Rendering|Components|Light|SetIntensity (Variables|Default|GetSpotLight) _lightintensity_alpha_3)
                    (Variables|Default|SetCurrentIntensity 0.0)
                    (Variables|Default|SetIsFadeActive? true))
                  (:Finished
                    (Variables|Default|SetIsFadeActive? false :!label _label_6)
                    (Utilities|FlowControl|Delay (Math|Random|RandomFloatinRange 0.0 0.6))
                    (goto _label_5 Reset)))
                (else
                  (Components|Timeline|SetTimelineLength (Variables|Default|GetFadeToLit_TL) (Math|Random|RandomFloatinRange 0.1 0.6))
                  (bind _lightintensity_alpha_4 (Timeline|Timeline_0 PlayFromStart)
                    (:Update
                      (Rendering|Components|Light|SetIntensity (Variables|Default|GetSpotLight) _lightintensity_alpha_4)
                      (Variables|Default|SetCurrentIntensity (Variables|Default|GetMaxLightIntensity))
                      (Variables|Default|SetIsFadeActive? true))
                    (:Finished
                      (goto _label_6))))))))))))

(event EventBeginPlay
  (|CallParentFunction)
  (CallFunction|LightFlicker))

(event Collision|EventActorBeginOverlap
  (params (OtherActor :type Actor%20Object%20Reference)))

(event EventTick
  (params (DeltaSeconds :type Float%20%28single-precision%29)))

(event EventTurnonLights
  ;[1 0 1] Turn On Lights
  (switch Utilities|FlowControl|Switch|SwitchonE_LightType (Variables|Default|GetLightType)
    (:NewEnumerator1
      (Rendering|SetVisibility (Variables|Default|GetPointLight) true false)
      (Rendering|SetVisibility (Variables|Default|GetSpotLight) false false))
    (:NewEnumerator2
      (Rendering|SetVisibility (Variables|Default|GetSpotLight) true false)
      (Rendering|SetVisibility (Variables|Default|GetRectLight) false false))
    (:NewEnumerator3
      (Rendering|SetVisibility (Variables|Default|GetRectLight) true false)
      (Rendering|SetVisibility (Variables|Default|GetSpotLight) false false)))
  (CallFunction|LightFlicker))

(event EventTurnOffLights
  ;[1 0 1] Turn Off Lights
  (Variables|Default|SetIsLightOn? false)
  (Rendering|SetVisibility (Variables|Default|GetSpotLight) false false))

(fn ConstructionScript
  (|CallParentFunction)
  (switch Utilities|FlowControl|Switch|SwitchonE_LightType (Variables|Default|GetLightType)
    (:NewEnumerator1
      (if (Variables|Default|GetIsLightOn?)
        (Rendering|SetVisibility (Variables|Default|GetPointLight) true false)
        (Rendering|SetVisibility (Variables|Default|GetSpotLight) false false)
        (else
          (Rendering|SetVisibility (Variables|Default|GetSpotLight) false false))))
    (:NewEnumerator2
      (if (Variables|Default|GetIsLightOn?)
        (Rendering|SetVisibility (Variables|Default|GetSpotLight) true false)
        (Rendering|SetVisibility (Variables|Default|GetRectLight) false false)
        (else
          (Rendering|SetVisibility (Variables|Default|GetSpotLight) false false))))
    (:NewEnumerator3
      (if (Variables|Default|GetIsLightOn?)
        (Rendering|SetVisibility (Variables|Default|GetRectLight) true false)
        (Rendering|SetVisibility (Variables|Default|GetSpotLight) false false)
        (else
          (Rendering|SetVisibility (Variables|Default|GetSpotLight) false false))))))