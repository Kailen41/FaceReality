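; BP_BaseLight is a light actor that can act as a point, spot or rect light and be turned on or off.
; The construction script shows the component matching LightType when IsLightOn is set and hides the other components.
; TurnOffLights clears IsLightOn and hides all three components.
; TurnonLights reapplies the LightType visibility but does not set IsLightOn back to true.
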(event EventBeginPlay
  (|CallParentFunction) ; This node is disabled and will not be called.\nDrag off pins to build functionality.
)

(event Collision|EventActorBeginOverlap
  (params (OtherActor :type Actor%20Object%20Reference)))

(event EventTick
  (params (DeltaSeconds :type Float%20%28single-precision%29)))

(event EventTurnonLights
  ;[1 0 1] Turn On Lights
  (switch Utilities|FlowControl|Switch|SwitchonE_LightType (Variables|Default|GetLightType)
    (:NewEnumerator1
      (Rendering|SetVisibility (Variables|Default|GetPointLight) true false)
      (Rendering|SetVisibility (Variables|Default|GetSpotLight) false false))
    (:NewEnumerator2
      (Rendering|SetVisibility (Variables|Default|GetSpotLight) true false)
      (Rendering|SetVisibility (Variables|Default|GetRectLight) false false))
    (:NewEnumerator3
      (Rendering|SetVisibility (Variables|Default|GetRectLight) true false)
      (Rendering|SetVisibility (Variables|Default|GetSpotLight) false false))))

(event EventTurnOffLights
  ;[1 0 1] Turn Off Lights
  (Variables|Default|SetIsLightOn? false)
  (Rendering|SetVisibility (Variables|Default|GetSpotLight) false false))

(fn ConstructionScript
  (|CallParentFunction)
  (switch Utilities|FlowControl|Switch|SwitchonE_LightType (Variables|Default|GetLightType)
    (:NewEnumerator1
      (if (Variables|Default|GetIsLightOn?)
        (Rendering|SetVisibility (Variables|Default|GetPointLight) true false)
        (Rendering|SetVisibility (Variables|Default|GetSpotLight) false false)
        (else
          (Rendering|SetVisibility (Variables|Default|GetSpotLight) false false))))
    (:NewEnumerator2
      (if (Variables|Default|GetIsLightOn?)
        (Rendering|SetVisibility (Variables|Default|GetSpotLight) true false)
        (Rendering|SetVisibility (Variables|Default|GetRectLight) false false)
        (else
          (Rendering|SetVisibility (Variables|Default|GetSpotLight) false false))))
    (:NewEnumerator3
      (if (Variables|Default|GetIsLightOn?)
        (Rendering|SetVisibility (Variables|Default|GetRectLight) true false)
        (Rendering|SetVisibility (Variables|Default|GetSpotLight) false false)
        (else
          (Rendering|SetVisibility (Variables|Default|GetSpotLight) false false))))))