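; BP_BaseKey is the base Blueprint for key items that the player picks up by interacting with them.
; Its Interact event increments the player's KeysHeld count, calls the player's key count update and crosshair clear, and adds its KeyID to KeyIDsHeld.
; The key then destroys itself, leaving the player to track both the total and the specific IDs held.
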(event EventBeginPlay)

(event Collision|EventActorBeginOverlap
  (params (OtherActor :type Actor%20Object%20Reference)))

(event EventTick
  (params (DeltaSeconds :type Float%20%28single-precision%29)))

(event EventInteract
  (bind _player_ref (Variables|Default|GetPlayer_REF))
  (Variables|/Game/_Main/MyBlueprints/Player/BP_Player.BP_Player_C|SetKeysHeld _player_ref (+ (Variables|/Game/_Main/MyBlueprints/Player/BP_Player.BP_Player_C|GetKeysHeld _player_ref) 1))
  (Default|CallUpdateKeysHeld (Variables|Default|GetPlayer_REF))
  (Default|CallCrosshairClear (Variables|Default|GetPlayer_REF))
  (Utilities|Array|Add (Variables|/Game/_Main/MyBlueprints/Player/BP_Player.BP_Player_C|GetKeyIDsHeld (Variables|Default|GetPlayer_REF)) (Variables|Default|GetKeyID))
  (Actor|DestroyActor))

(fn ConstructionScript
  (|CallParentFunction))