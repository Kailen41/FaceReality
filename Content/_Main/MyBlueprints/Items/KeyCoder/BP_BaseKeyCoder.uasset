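; Base interactable keypad that unlocks a locked door when the player enters the correct four-digit code.
; Interact toggles, behind a short cooldown, between a blended keypad view with mouse cursor and frozen movement, and normal play.
; Clicked buttons animate and feed digits to a screen widget, whose input is checked against the required code.
; Failure resets entry; success calls unlock with DoorToUnlock on the BP_BaseLockedDoor found through GetActorOfClass.
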(event OnClicked(Button1)
  (params (TouchedComponent :type Primitive%20Component%20Object%20Reference) (ButtonPressed :type Key%20Structure :default "None"))
  ;[1 0 1] Input for buttons for the key coder
  (if (== ButtonPressed "LeftMouseButton")
    (CallFunction|AnimateKeyCoderButton (Variables|Default|GetButton1))
    (Utilities|UpdateKeyCoderCode 1
      (:Success
        (Default|CallUnlockDoor (Variables|Default|GetBaseLockedDoor_REF) (Variables|Default|GetDoorToUnlock))))))

(event OnClicked(Button5)
  (params (TouchedComponent :type Primitive%20Component%20Object%20Reference) (ButtonPressed :type Key%20Structure :default "None"))
  ;[1 0 1] Input for buttons for the key coder
  (if (== ButtonPressed "LeftMouseButton")
    (CallFunction|AnimateKeyCoderButton (Variables|Default|GetButton5))
    (Utilities|UpdateKeyCoderCode 5
      (:Success
        (Default|CallUnlockDoor (Variables|Default|GetBaseLockedDoor_REF) (Variables|Default|GetDoorToUnlock))))))

(event OnClicked(Button6)
  (params (TouchedComponent :type Primitive%20Component%20Object%20Reference) (ButtonPressed :type Key%20Structure :default "None"))
  ;[1 0 1] Input for buttons for the key coder
  (if (== ButtonPressed "LeftMouseButton")
    (CallFunction|AnimateKeyCoderButton (Variables|Default|GetButton6))
    (Utilities|UpdateKeyCoderCode 6
      (:Success
        (Default|CallUnlockDoor (Variables|Default|GetBaseLockedDoor_REF) (Variables|Default|GetDoorToUnlock))))))

(event OnClicked(Button7)
  (params (TouchedComponent :type Primitive%20Component%20Object%20Reference) (ButtonPressed :type Key%20Structure :default "None"))
  ;[1 0 1] Input for buttons for the key coder
  (if (== ButtonPressed "LeftMouseButton")
    (CallFunction|AnimateKeyCoderButton (Variables|Default|GetButton7))
    (Utilities|UpdateKeyCoderCode 7
      (:Success
        (Default|CallUnlockDoor (Variables|Default|GetBaseLockedDoor_REF) (Variables|Default|GetDoorToUnlock))))))

(event OnClicked(Button8)
  (params (TouchedComponent :type Primitive%20Component%20Object%20Reference) (ButtonPressed :type Key%20Structure :default "None"))
  ;[1 0 1] Input for buttons for the key coder
  (if (== ButtonPressed "LeftMouseButton")
    (CallFunction|AnimateKeyCoderButton (Variables|Default|GetButton8))
    (Utilities|UpdateKeyCoderCode 8
      (:Success
        (Default|CallUnlockDoor (Variables|Default|GetBaseLockedDoor_REF) (Variables|Default|GetDoorToUnlock))))))

(event OnClicked(Button2)
  (params (TouchedComponent :type Primitive%20Component%20Object%20Reference) (ButtonPressed :type Key%20Structure :default "None"))
  ;[1 0 1] Input for buttons for the key coder
  (if (== ButtonPressed "LeftMouseButton")
    (CallFunction|AnimateKeyCoderButton (Variables|Default|GetButton2))
    (Utilities|UpdateKeyCoderCode 2
      (:Success
        (Default|CallUnlockDoor (Variables|Default|GetBaseLockedDoor_REF) (Variables|Default|GetDoorToUnlock))))))

(event OnClicked(Button9)
  (params (TouchedComponent :type Primitive%20Component%20Object%20Reference) (ButtonPressed :type Key%20Structure :default "None"))
  ;[1 0 1] Input for buttons for the key coder
  (if (== ButtonPressed "LeftMouseButton")
    (CallFunction|AnimateKeyCoderButton (Variables|Default|GetButton9))
    (Utilities|UpdateKeyCoderCode 9
      (:Success
        (Default|CallUnlockDoor (Variables|Default|GetBaseLockedDoor_REF) (Variables|Default|GetDoorToUnlock))))))

(event OnClicked(Button0)
  (params (TouchedComponent :type Primitive%20Component%20Object%20Reference) (ButtonPressed :type Key%20Structure :default "None"))
  ;[1 0 1] Input for buttons for the key coder
  (if (== ButtonPressed "LeftMouseButton")
    (CallFunction|AnimateKeyCoderButton (Variables|Default|GetButton0))
    (Utilities|UpdateKeyCoderCode
      (:Success
        (Default|CallUnlockDoor (Variables|Default|GetBaseLockedDoor_REF) (Variables|Default|GetDoorToUnlock))))))

(event OnClicked(Button3)
  (params (TouchedComponent :type Primitive%20Component%20Object%20Reference) (ButtonPressed :type Key%20Structure :default "None"))
  ;[1 0 1] Input for buttons for the key coder
  (if (== ButtonPressed "LeftMouseButton")
    (CallFunction|AnimateKeyCoderButton (Variables|Default|GetButton3))
    (Utilities|UpdateKeyCoderCode 3
      (:Success
        (Default|CallUnlockDoor (Variables|Default|GetBaseLockedDoor_REF) (Variables|Default|GetDoorToUnlock))))))

(event OnClicked(Button4)
  (params (TouchedComponent :type Primitive%20Component%20Object%20Reference) (ButtonPressed :type Key%20Structure :default "None"))
  ;[1 0 1] Input for buttons for the key coder
  (if (== ButtonPressed "LeftMouseButton")
    (CallFunction|AnimateKeyCoderButton (Variables|Default|GetButton4))
    (Utilities|UpdateKeyCoderCode 4
      (:Success
        (Default|CallUnlockDoor (Variables|Default|GetBaseLockedDoor_REF) (Variables|Default|GetDoorToUnlock))))))

(event Custom|AnimateKeyCoderButton
  (params (Button :type Scene%20Component%20Object%20Reference))
  ;[1 0 1] Button animation
  (Audio|PlaySound2D "/Game/_Main/Audio/FX/KeyCoderClick_Cue.KeyCoderClick_Cue" 1.0 1.0 0.0 0 0)
  (bind _location_alpha (Timeline|ButtonAnim_TL PlayFromStart)
    (:Update
      (Transformation|SetRelativeRotation Button (Math|Rotator|MakeRotator 0.0 _location_alpha 0.0) false false))))

(event EventBeginPlay
  ;[0 0 1] BeginPlay
  (|CallParentFunction)
  (bind _aswbp_key_coder_screen (Utilities|Casting|CastToWBP_KeyCoderScreen (UserInterface|GetWidget (Variables|Default|GetScreenNumbersWidget))))
  (Variables|Default|SetKeyCoderScreenWidget_REF _aswbp_key_coder_screen)
  (bind _returnvalue (Actor|GetActorOfClass "/Game/_Main/MyBlueprints/Items/Environmental/Doors/LockedDoors/BP_BaseLockedDoor.BP_BaseLockedDoor_C"))
  (Variables|Default|SetBaseLockedDoor_REF _returnvalue))

(event EventTick
  (params (DeltaSeconds :type Float%20%28single-precision%29)))

(event EventInteract
  (bind _returnvalue (Game|GetPlayerController 0))
  (bind _returnvalue_2 (Game|GetPlayerController 0))
  (bind _screennumberswidget (Variables|Default|GetScreenNumbersWidget))
  (bind _returnvalue_3 (UserInterface|GetWidget _screennumberswidget))
  (Utilities|FlowControl|DoOnce false :!label _label
    (:Completed
      (Utilities|FlowControl|FlipFlop
        (:A
          (Game|Player|SetViewTargetwithBlend (Game|GetPlayerController 0) self 0.3 "VTBlend_Linear" 0.0 false)
          (Widget|SetVisibility (Variables|/Game/_Main/MyBlueprints/Widgets/WBP_HUD.WBP_HUD_C|GetCrosshairBorder (Variables|/Game/_Main/MyBlueprints/Player/BP_Player.BP_Player_C|GetHUD_REF (Variables|Default|GetPlayer_REF))) "Hidden")
          (Audio|PlaySound2D "/Game/_Main/Audio/FX/KeyCoderActivate_Cue.KeyCoderActivate_Cue" 1.0 1.0 0.0 0 0)
          (Pawn|Components|CharacterMovement|SetMovementMode (Variables|/Script/Engine.Character|GetCharacterMovement (Variables|Default|GetPlayer_REF)) "MOVE_None" 0)
          (Variables|/Script/Engine.PlayerController|SetbShowMouseCursor _returnvalue true)
          (Input|SetInputModeGameandUI _returnvalue _returnvalue_3 "DoNotLock" true false)
          (Class|BPIKeyCoder|SetCurrentKeyCoder(Message) _returnvalue_3 self)
          (Utilities|FlowControl|Delay 0.3)
          (goto _label Reset))
        (:B
          (Game|Player|SetViewTargetwithBlend (Game|GetPlayerController 0) (Variables|Default|GetPlayer_REF) 0.3 "VTBlend_Linear" 0.0 false)
          (Widget|SetVisibility (Variables|/Game/_Main/MyBlueprints/Widgets/WBP_HUD.WBP_HUD_C|GetCrosshairBorder (Variables|/Game/_Main/MyBlueprints/Player/BP_Player.BP_Player_C|GetHUD_REF (Variables|Default|GetPlayer_REF))) "Visible")
          (Audio|PlaySound2D "/Game/_Main/Audio/FX/KeyCoderActivate_Cue.KeyCoderActivate_Cue" 1.0 1.0 0.0 0 0)
          (Pawn|Components|CharacterMovement|SetMovementMode (Variables|/Script/Engine.Character|GetCharacterMovement (Variables|Default|GetPlayer_REF)) "MOVE_Walking" 0)
          (Variables|/Script/Engine.PlayerController|SetbShowMouseCursor _returnvalue_2 false)
          (Input|SetInputModeGameOnly _returnvalue_2 false)
          (Utilities|FlowControl|Delay 0.3)
          (goto _label Reset))))))

(fn ConstructionScript
  (|CallParentFunction))