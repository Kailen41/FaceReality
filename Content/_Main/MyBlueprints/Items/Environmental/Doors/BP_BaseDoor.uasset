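; BP_BaseDoor is a base environmental door actor whose look and item info come from a data table.
; The construction script reads the DoorName row handle, stores the row as ItemInfo and sets the Door static mesh from it.
; On BeginPlay it casts the player character to BP_FirstPersonCharacter and caches it as PlayerREF.
; No opening or interaction logic is present in its graphs.
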(event EventBeginPlay
  (bind _asbp_first_person_character (Utilities|Casting|CastToBP_FirstPersonCharacter (Game|GetPlayerCharacter 0)))
  (Variables|Default|SetPlayer_REF _asbp_first_person_character))

(event Collision|EventActorBeginOverlap
  (params (OtherActor :type Actor%20Object%20Reference)))

(event EventTick
  (params (DeltaSeconds :type Float%20%28single-precision%29)))

(fn ConstructionScript
  (bind _doorname (Variables|Default|GetDoorName))
  (bind (_datatable _rowname) (Utilities|Struct|BreakDataTableRowHandle _doorname))
  (bind _returnvalue (Utilities|GetDataTableRow _datatable _rowname)
    (:then
      (bind _output_get (Variables|Default|SetItemInfo _returnvalue))
      (Components|StaticMesh|SetStaticMesh (Variables|Default|GetDoor) (.StaticMesh (Utilities|Struct|BreakS_ItemInfo _output_get))))))