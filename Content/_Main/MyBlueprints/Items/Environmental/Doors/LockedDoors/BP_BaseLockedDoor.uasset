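; Base interactable locked door that swings on a hinge and can require player-held keys.
; Interacting with a Key Door spends a key, optionally matching and removing a required ID, then unlocks and toggles it.
; DoOnce-guarded timelines drive the hinge with sounds, optionally using a door-player dot product to choose swing direction.
; An UnlockDoor dispatcher bound on BeginPlay also unlocks the door when it is the target.
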(event Custom|UnlockDoorEvent
  (EventDispatchers|BindEventtoUnlockDoor (delegate Custom|UnlockDoorEventBind)))

(event Custom|UnlockDoorEventBind
  (params (DoorToUnlock :type Actor%20Object%20Reference))
  (if (== DoorToUnlock self)
    (Variables|Booleans|SetIsDoorUnlocked? true)))

(event Collision|EventActorBeginOverlap
  (params (OtherActor :type Actor%20Object%20Reference))
  (|CallParentFunction OtherActor) ; This node is disabled and will not be called.\nDrag off pins to build functionality.
)

(event EventTick
  (params (DeltaSeconds :type Float%20%28single-precision%29))
  (|CallParentFunction DeltaSeconds) ; This node is disabled and will not be called.\nDrag off pins to build functionality.
)

(event EventInteract
  (bind _player_ref (Variables|Default|GetPlayer_REF))
  (switch Utilities|FlowControl|Switch|SwitchonE_DoorType (.DoorType (Utilities|Struct|BreakS_DoorInfo (Utilities|Struct|BreakS_ItemInfo (Variables|Default|GetItemInfo))))
    (:NewEnumerator2
      (if (Variables|Booleans|GetIsDoorUnlocked?)
        (if (Variables|Default|GetUseDOT?) :!label _label
          (bind _output_get (Variables|Default|SetDirection (Math|Float|Round (Math|Vector|DotProduct (Math|Vector|GetForwardVector (Transformation|GetActorRotation)) (Math|Vector|GetRightVector (Transformation|GetActorRotation (Game|GetPlayerCharacter 0)))))))
          (if (not (== _output_get 0))
            (if (Variables|Default|GetIsDoorOpen?)
              (Utilities|FlowControl|DoOnce false :!label _label_2
                (:Completed
                  (Audio|PlaySound2D "/Game/DoorSFX/SoundCue/Drs_Front_Door_Close_02_Cue.Drs_Front_Door_Close_02_Cue" 1.0 1.0 0.0 0 0)
                  (if (== (Variables|Default|GetDOTDoorAngle_REF) -9e+01)
                    (bind _doorangle_alpha (Timeline|Timeline_0 PlayFromStart)
                      (:Update
                        (Transformation|SetRelativeRotation (Variables|Default|GetHinge) (Math|Rotator|MakeRotator 0.0 0.0 _doorangle_alpha) false false))
                      (:Finished
                        (Variables|Default|SetIsDoorOpen? false)
                        (goto _label_2 Reset)))
                    (else
                      (bind _doorangle_alpha_2 (Timeline|Timeline_1 PlayFromStart)
                        (:Update
                          (Transformation|SetRelativeRotation (Variables|Default|GetHinge) (Math|Rotator|MakeRotator 0.0 0.0 _doorangle_alpha_2) false false))
                        (:Finished
                          (Variables|Default|SetIsDoorOpen? false)
                          (goto _label_2 Reset)))))))
              (else
                (Utilities|FlowControl|DoOnce false :!label _label_3
                  (:Completed
                    (Audio|PlaySound2D "/Game/DoorSFX/SoundCue/Drs_Front_Door_Open_02_Cue.Drs_Front_Door_Open_02_Cue" 1.0 1.0 0.0 0 0)
                    (bind _doorangle_alpha_3 (Timeline|Timeline PlayFromStart)
                      (:Update
                        (Variables|Default|SetDOTDoorAngle_REF (* _doorangle_alpha_3 (Variables|Default|GetDirection)))
                        (Transformation|SetRelativeRotation (Variables|Default|GetHinge) (Math|Rotator|MakeRotator 0.0 0.0 (* _doorangle_alpha_3 (Variables|Default|GetDirection))) false false))
                      (:Finished
                        (Variables|Default|SetIsDoorOpen? true)
                        (goto _label_3 Reset))))))))
          (elif (Variables|Default|GetIsDoorOpen?)
            (Utilities|FlowControl|DoOnce false :!label _label_4
              (:Completed
                (Audio|PlaySound2D "/Game/DoorSFX/SoundCue/Drs_Front_Door_Close_02_Cue.Drs_Front_Door_Close_02_Cue" 1.0 1.0 0.0 0 0)
                (bind _doorangle_alpha_4 (Timeline|DoorClose_TL PlayFromStart)
                  (:Update
                    (Transformation|SetRelativeRotation (Variables|Default|GetHinge) (Math|Rotator|MakeRotator 0.0 0.0 _doorangle_alpha_4) false false))
                  (:Finished
                    (Variables|Default|SetIsDoorOpen? false)
                    (goto _label_4 Reset)))))
            (else
              (Utilities|FlowControl|DoOnce false :!label _label_5
                (:Completed
                  (Audio|PlaySound2D "/Game/DoorSFX/SoundCue/Drs_Front_Door_Open_02_Cue.Drs_Front_Door_Open_02_Cue" 1.0 1.0 0.0 0 0)
                  (bind _doorangle_alpha_5 (Timeline|DoorOpen_TL PlayFromStart)
                    (:Update
                      (Transformation|SetRelativeRotation (Variables|Default|GetHinge) (Math|Rotator|MakeRotator 0.0 0.0 _doorangle_alpha_5) false false))
                    (:Finished
                      (Variables|Default|SetIsDoorOpen? true)
                      (goto _label_5 Reset))))))))
        (elif (Variables|Booleans|GetIsIDRequired?)
          (bind _array_element (Utilities|Array|ForEachLoopwithBreak (Variables|/Game/_Main/MyBlueprints/Player/BP_Player.BP_Player_C|GetKeyIDsHeld (Variables|Default|GetPlayer_REF)) :!label _label_6)
            (:LoopBody
              (if (== _array_element (Variables|Default|GetIDRequired))
                (Variables|Booleans|SetIsIDFound? true)
                (goto _label_6 Break)))
            (:Completed
              (if (Variables|Booleans|GetIsIDFound?)
                (Utilities|Array|RemoveItem (Variables|/Game/_Main/MyBlueprints/Player/BP_Player.BP_Player_C|GetKeyIDsHeld (Variables|Default|GetPlayer_REF)) (Variables|Default|GetIDRequired))
                (if (> (Variables|/Game/_Main/MyBlueprints/Player/BP_Player.BP_Player_C|GetKeysHeld (Variables|Default|GetPlayer_REF)) 0) :!label _label_7
                  (Variables|/Game/_Main/MyBlueprints/Player/BP_Player.BP_Player_C|SetKeysHeld _player_ref (Math|Integer|Clamp(Integer) (- (Variables|/Game/_Main/MyBlueprints/Player/BP_Player.BP_Player_C|GetKeysHeld _player_ref) 1) 0 99))
                  (Default|CallUpdateKeysHeld (Variables|Default|GetPlayer_REF))
                  (Variables|Booleans|SetIsDoorUnlocked? true)
                  (goto _label)))))
          (else
            (goto _label_7)))))))

(event EventBeginPlay
  (|CallParentFunction)
  (CallFunction|UnlockDoorEvent))

(fn ConstructionScript
  (|CallParentFunction))