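; Base interactable light switch that toggles the lights listed in LightsToEffect.
; Interact plays the item's pickup sound, then sends on or off messages to each light based on IsLightsOn.
; The state flip and Switch roll timelines run inside each loop, so an empty list never toggles.
; The construction script matches the switch tilt and light states to the initial IsLightsOn value.
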(event EventBeginPlay
  (|CallParentFunction) ; This node is disabled and will not be called.\nDrag off pins to build functionality.
)

(event Collision|EventActorBeginOverlap
  (params (OtherActor :type Actor%20Object%20Reference)))

(event EventTick
  (params (DeltaSeconds :type Float%20%28single-precision%29)))

(event EventInteract
  (Audio|PlaySound2D (Utilities|Struct|BreakS_ItemInfo (Variables|Default|GetItemInfo)) 1.0 1.0 0.0 0 0)
  (if (Variables|Default|GetIsLightsOn?)
    (for _array_element (Variables|Default|GetLightsToEffect)
      (Class|BPILights|TurnOffLights(Message) _array_element)
      (Variables|Default|SetIsLightsOn? false)
      (bind _turnonrotation_alpha (Timeline|TurnOff_TL PlayFromStart)
        (:Update
          (Transformation|SetRelativeRotation (Variables|Default|GetSwitch) (Math|Rotator|MakeRotator _turnonrotation_alpha 0.0 0.0) false false))))
    (else
      (for _array_element_2 (Variables|Default|GetLightsToEffect)
        (Class|BPILights|TurnonLights(Message) _array_element_2)
        (Variables|Default|SetIsLightsOn? true)
        (bind _turnoffrotation_alpha (Timeline|TurnOn_TL PlayFromStart)
          (:Update
            (Transformation|SetRelativeRotation (Variables|Default|GetSwitch) (Math|Rotator|MakeRotator _turnoffrotation_alpha 0.0 0.0) false false)))))))

(fn ConstructionScript
  (bind _lightstoeffect (Variables|Default|GetLightsToEffect))
  (|CallParentFunction)
  (if (Variables|Default|GetIsLightsOn?)
    (Transformation|SetRelativeRotation (Variables|Default|GetSwitch) (Math|Rotator|MakeRotator -3e+01 0.0 0.0) false false)
    (for _array_element _lightstoeffect
      (Class|BPILights|TurnonLights(Message) _array_element))
    (else
      (Transformation|SetRelativeRotation (Variables|Default|GetSwitch) (Math|Rotator|MakeRotator 3e+01 0.0 0.0) false false)
      (for _array_element_2 _lightstoeffect
        (Class|BPILights|TurnOffLights(Message) _array_element_2)))))