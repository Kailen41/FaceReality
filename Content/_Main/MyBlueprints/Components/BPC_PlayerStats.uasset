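; Player stats component that handles sprint stamina for the first-person character.
; Looping timers drain stamina while the player moves and regenerate it up to max, asking the character to update stamina each tick.
; Sprinting stops when stamina empties or movement ceases, resetting walk speed and starting regeneration, with a short delay if fully depleted.
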(event Custom|AddStamina
  ;[1 0 1] Handles all stamina functionality
  ;;[0.04688 0.04688 0.04688] Adds Stamina
  (bind _returnvalue (Utilities|Time|SetTimerbyEvent (delegate Custom|AddStaminaTimer) 0.1 true))
  (Variables|Default|SetAddStaminaTimerHandle _returnvalue))

(event Custom|AddStaminaTimer
  ;[1 0 1] Handles all stamina functionality
  ;;[0.04688 0.04688 0.04688] Adds Stamina
  (Default|CallUpdateStamina (Variables|Default|GetPlayer_REF))
  (Variables|Default|SetCurrentStamina (Math|Float|Clamp(Float) (+ (Variables|Default|GetCurrentStamina) (Variables|Default|GetAddStaminaAmount)) 0.0 (Variables|Default|GetMaxStamina)))
  (if (== (Variables|Default|GetCurrentStamina) (Variables|Default|GetMaxStamina))
    (Utilities|Time|ClearandInvalidateTimerbyHandle (Variables|Default|GetAddStaminaTimerHandle))))

(event Custom|DrainStamina
  ;[1 0 1] Handles all stamina functionality
  ;;[0.04688 0.04688 0.04688] Drains Stamina
  (bind _returnvalue (Utilities|Time|SetTimerbyEvent (delegate Custom|DrainStaminaTimer) 0.1 true))
  (Variables|Default|SetDrainStaminaTimerHandle _returnvalue))

(event Custom|DrainStaminaTimer
  ;[1 0 1] Handles all stamina functionality
  ;;[0.04688 0.04688 0.04688] Drains Stamina
  (Utilities|Time|ClearandInvalidateTimerbyHandle (Variables|Default|GetAddStaminaTimerHandle))
  (if (Variables|/Game/FirstPerson/Blueprints/BP_FirstPersonCharacter.BP_FirstPersonCharacter_C|GetIsMoving? (Variables|Default|GetPlayer_REF))
    (Default|CallUpdateStamina (Variables|Default|GetPlayer_REF))
    (bind _output_get (Variables|Default|SetCurrentStamina (Math|Float|Clamp(Float) (- (Variables|Default|GetCurrentStamina) (Variables|Default|GetDrainStaminaAmount)) 0.0 (Variables|Default|GetMaxStamina))))
    (if (<= _output_get 0.0)
      (CallFunction|StopSprinting))
    (else
      (CallFunction|StopSprinting))))

(event Custom|StopSprinting
  ;[1 0 1] Handles all stamina functionality
  ;;[0.04688 0.04688 0.04688] Stops Sprinting
  (Default|FSetMaxWalkSpeed (Variables|Default|GetPlayer_REF) (Variables|Default|GetMaxWalkSpeed))
  (Variables|/Game/FirstPerson/Blueprints/BP_FirstPersonCharacter.BP_FirstPersonCharacter_C|SetIsSprint? (Variables|Default|GetPlayer_REF) false)
  (Utilities|Time|ClearandInvalidateTimerbyHandle (Variables|Default|GetDrainStaminaTimerHandle))
  (if (<= (Variables|Default|GetCurrentStamina) 0.0)
    (Utilities|FlowControl|Delay 1.0)
    (CallFunction|AddStamina)
    (else
      (CallFunction|AddStamina))))

(event EventBeginPlay
  ;[0 0 1] BeginPlay
  (bind _asbp_first_person_character (Utilities|Casting|CastToBP_FirstPersonCharacter (Game|GetPlayerCharacter 0)))
  (Variables|Default|SetPlayer_REF _asbp_first_person_character))